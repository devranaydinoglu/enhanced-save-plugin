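; Savable actor in the save system with a point light that turns on when the save character touches it.
; Overlapping its sphere with a BP_SaveCharacter sets IsLightOn and calls ChangeSavableVariableValues on that character.
; Tick applies IsLightOn to the light's visibility every frame, so the light always follows the variable.
; A delayed DestroyActor chain is left unconnected and never runs.
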(event OnComponentBeginOverlap(Sphere)
  (params (OverlappedComponent :type Primitive%20Component%20Object%20Reference) (OtherActor :type Actor%20Object%20Reference) (OtherComp :type Primitive%20Component%20Object%20Reference) (OtherBodyIndex :type Integer) (bFromSweep :type Boolean) (SweepResult :type Hit%20Result%20Structure%20%28by%20ref%29))
  ;[1 1 1] Turn light on on overlap
  (bind _asbp_save_character (Utilities|Casting|CastToBP_SaveCharacter OtherActor))
  (Variables|Default|SetbIsLightOn true)
  (Default|ChangeSavableVariableValues _asbp_save_character))

(event EventTick
  (params (DeltaSeconds :type Float%20%28single-precision%29))
  ;[1 1 1] Update light visibility
  (if (Variables|Default|GetbIsLightOn)
    (Rendering|SetVisibility (Variables|Default|GetPointLight) true false)
    (else
      (Rendering|SetVisibility (Variables|Default|GetPointLight) false false))))

(fn ConstructionScript)