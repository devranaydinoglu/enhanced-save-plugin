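; BP_SavePlayerState is a player state Blueprint that exercises the save system with a test float held on its BPSaveComponent.
; It prints a message on spawn and prints the component's float on the PreSaveGame and PostLoadGame events to show the saved and restored value.
; ChangeSavableVariableValues increments that float but is not called within this Blueprint.
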(event EventBeginPlay
  (Development|PrintString "PLAYER STATE SPAWNED"))

(event EventPreSaveGame
  (CallFunction|PrintSavableVariables))

(event EventPostLoadGame
  (CallFunction|PrintSavableVariables))

(fn ConstructionScript)

(fn ChangeSavableVariableValues
  (bind _bp_savecomponent (Variables|Default|GetBP_SaveComponent))
  (Variables|/Game/SaveSystem/Blueprints/BP_SaveComponent.BP_SaveComponent_C|SetFloatTest _bp_savecomponent (+ (Variables|/Game/SaveSystem/Blueprints/BP_SaveComponent.BP_SaveComponent_C|GetFloatTest _bp_savecomponent) 1.0)))

(fn PrintSavableVariables
  (Development|PrintString (Utilities|String|Append "PLAYER STATE CompTest:" (Utilities|String|ToString(Float) (Variables|/Game/SaveSystem/Blueprints/BP_SaveComponent.BP_SaveComponent_C|GetFloatTest (Variables|Default|GetBP_SaveComponent)))) true true "(R=0.000000,G=0.660000,B=1.000000,A=1.000000)" 8.0))