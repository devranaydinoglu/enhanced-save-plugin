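; Player character for testing world save and load through the ESS subsystem, with Enhanced Input movement, look and jump.
; Debug keys save, load or delete one slot and print the result; global-object save/load nodes are unwired.
; Save hooks print test variables of assorted types, including a component value, and post-load re-possesses the character.
; A helper, uncalled here, mutates those values plus GameMode and GameInstance fields.
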(event Input|EnhancedActionEvents|EnhancedInputActionIA_Move
  (params (ActionValue :type Vector%202D%20Structure) (ElapsedSeconds :type Float%20%28double-precision%29) (TriggeredSeconds :type Float%20%28double-precision%29) (InputAction :type Input%20Action%20Object%20Reference :default "/Game/SaveSystem/Input/IA_Move.IA_Move"))
  (bind _returnvalue (Pawn|GetControlRotation :!class /Script/Engine.Pawn))
  ;[0.1198 0.1198 0.1198] Input
  (Pawn|Input|AddMovementInput (Math|Vector|GetRightVector (Math|Rotator|MakeRotator (.roll _returnvalue) 0.0 (.yaw _returnvalue))) (.x ActionValue) false)
  (Pawn|Input|AddMovementInput (Math|Vector|GetForwardVector (Math|Rotator|MakeRotator 0.0 0.0 (.yaw (Pawn|GetControlRotation :!class /Script/Engine.Pawn)))) (.y ActionValue) false))

(event Input|EnhancedActionEvents|EnhancedInputActionIA_Jump
  (params (ActionValue :type Boolean) (ElapsedSeconds :type Float%20%28double-precision%29) (TriggeredSeconds :type Float%20%28double-precision%29) (InputAction :type Input%20Action%20Object%20Reference :default "/Game/SaveSystem/Input/IA_Jump.IA_Jump"))
  ;[0.1198 0.1198 0.1198] Input
  (:Triggered
    (Character|Jump))
  (:Canceled
    (Character|StopJumping :!label _label))
  (:Completed
    (goto _label)))

(event Input|EnhancedActionEvents|EnhancedInputActionIA_Look
  (params (ActionValue :type Vector%202D%20Structure) (ElapsedSeconds :type Float%20%28double-precision%29) (TriggeredSeconds :type Float%20%28double-precision%29) (InputAction :type Input%20Action%20Object%20Reference :default "/Game/SaveSystem/Input/IA_Look.IA_Look"))
  ;[0.1198 0.1198 0.1198] Input
  (Pawn|Input|AddControllerYawInput (.x ActionValue))
  (Pawn|Input|AddControllerPitchInput (.y ActionValue)))

(event EventBeginPlay
  (Utilities|FlowControl|Sequence
    (:then_0
      (bind _asbp_save_controller (Utilities|Casting|CastToBP_SaveController (Pawn|GetController)))
      (Input|AddMappingContext (PlayerController|LocalPlayerSubsystems|GetEnhancedInputLocalPlayerSubsystem _asbp_save_controller) "/Game/SaveSystem/Input/IMC_Default.IMC_Default" 0 "(bIgnoreAllPressedKeysUntilRelease=True,bForceImmediately=False,bNotifyUserSettings=False)"))
    (:then_1
      (bind _asbp_save_game_mode (Utilities|Casting|CastToBP_SaveGameMode (Game|GetGameMode)))
      (Variables|Default|SetGameMode _asbp_save_game_mode)
      (bind _asbp_save_game_instance (Utilities|Casting|CastToBP_SaveGameInstance (Game|GetGameInstance)))
      (Variables|Default|SetGameInstance _asbp_save_game_instance))))

(event EventPostLoadGame
  (Pawn|Possess (Game|GetPlayerController 0) self)
  (CallFunction|PrintSavableVariables))

(event EventPreSaveGame
  (CallFunction|PrintSavableVariables))

(event Input|KeyboardEvents|F
  (params (Key :type Key%20Structure :default "None"))
  (:Pressed
    (bind _returnvalue (Class|EssSubsystem|SaveWorld (Subsystems|GetEssSubsystem) "Slot1"))
    (Development|PrintString (Utilities|String|Append "Game saved: " (Utilities|String|ToString(Boolean) _returnvalue)))))

(event Input|KeyboardEvents|G
  (params (Key :type Key%20Structure :default "None"))
  (:Pressed
    (bind _returnvalue (Class|EssSubsystem|LoadWorld (Subsystems|GetEssSubsystem) "Slot1"))
    (Development|PrintString (Utilities|String|Append "Game loaded: " (Utilities|String|ToString(Boolean) _returnvalue)))))

(event Input|KeyboardEvents|Q
  (params (Key :type Key%20Structure :default "None"))
  (:Pressed
    (bind _returnvalue (SaveGame|DeleteGameinSlot "Slot1"))
    (Development|PrintString (Utilities|String|Append "Save slot deleted: " (Utilities|String|ToString(Boolean) _returnvalue)))))

(fn ConstructionScript)

(fn PrintSavableVariables
  (bind _structtest (Variables|Default|GetStructTest))
  (Development|PrintString (Utilities|String|Append "BoolTest:" (Utilities|String|ToString(Boolean) (Variables|Default|GetbBoolTest))) true true "(R=0.000000,G=0.660000,B=1.000000,A=1.000000)" 8.0)
  (Development|PrintString (Utilities|String|Append "IntTest:" (Utilities|String|ToString(Integer) (Variables|Default|GetIntTest))) true true "(R=0.000000,G=0.660000,B=1.000000,A=1.000000)" 8.0)
  (Development|PrintString (Utilities|String|Append "StringTest:" (Variables|Default|GetStringTest)) true true "(R=0.000000,G=0.660000,B=1.000000,A=1.000000)" 8.0)
  (Development|PrintString (Utilities|String|Append "VectorTest:" (Utilities|String|ToString(Vector) (Variables|Default|GetVectorTest))) true true "(R=0.000000,G=0.660000,B=1.000000,A=1.000000)" 8.0)
  (Development|PrintString (Utilities|String|Append "EnumTest:" (Utilities|String|EnumtoString (Variables|Default|GetEnumTest))) true true "(R=0.000000,G=0.660000,B=1.000000,A=1.000000)" 8.0)
  (Development|PrintString (Utilities|String|Append (Utilities|String|Append (Utilities|String|Append "Float: " (Utilities|String|ToString(Float) (.floattest _structtest))) (Utilities|String|Append "Text: " (Utilities|String|ToString(Text) (.texttest _structtest)))) (Utilities|String|Append "Rotator:" (Utilities|String|ToString(Rotator) (.rotatortest _structtest)))) true true "(R=0.000000,G=0.660000,B=1.000000,A=1.000000)" 8.0)
  (Development|PrintString (Utilities|String|Append "CompTest:" (Utilities|String|ToString(Float) (Variables|/Game/SaveSystem/Blueprints/BP_SaveComponent.BP_SaveComponent_C|GetFloatTest (Variables|Default|GetBP_SaveComponent)))) true true "(R=0.000000,G=0.660000,B=1.000000,A=1.000000)" 8.0))

(fn ChangeSavableVariableValues
  (bind _bp_savecomponent (Variables|Default|GetBP_SaveComponent))
  (bind _gamemode (Variables|Default|GetGameMode))
  (bind _gameinstance (Variables|Default|GetGameInstance))
  (Variables|Default|SetbBoolTest (not (Variables|Default|GetbBoolTest)))
  (Variables|Default|SetIntTest (+ (Variables|Default|GetIntTest) 1))
  (Variables|Default|SetStringTest (Utilities|String|Append (Variables|Default|GetStringTest) "a"))
  (Variables|Default|SetVectorTest (Math|Vector|MakeVector (+ (.x (Variables|Default|GetVectorTest)) 5.0) 0.0 0.0))
  (Variables|Default|SetStructTest (Utilities|Struct|MakeS_SaveStruct (+ (.floattest (Variables|Default|GetStructTest)) 1.0) (Utilities|Text|ToText(String) (Utilities|String|Append (Utilities|String|ToString(Text) (.texttest (Variables|Default|GetStructTest))) "a")) (Math|Rotator|MakeRotator (+ (.Roll (Math|Rotator|BreakRotator (.rotatortest (Variables|Default|GetStructTest)))) 5.0) 0.0 0.0)))
  (Variables|Default|SetEnumTest "NewEnumerator0")
  (Variables|/Game/SaveSystem/Blueprints/BP_SaveGameMode.BP_SaveGameMode_C|SetFloatTest _gamemode (+ (Variables|/Game/SaveSystem/Blueprints/BP_SaveGameMode.BP_SaveGameMode_C|GetFloatTest _gamemode) 1.0))
  (Variables|/Game/SaveSystem/Blueprints/BP_SaveGameInstance.BP_SaveGameInstance_C|SetIntTest _gameinstance (+ (Variables|/Game/SaveSystem/Blueprints/BP_SaveGameInstance.BP_SaveGameInstance_C|GetIntTest _gameinstance) 1))
  (Variables|/Game/SaveSystem/Blueprints/BP_SaveComponent.BP_SaveComponent_C|SetFloatTest _bp_savecomponent (+ (Variables|/Game/SaveSystem/Blueprints/BP_SaveComponent.BP_SaveComponent_C|GetFloatTest _bp_savecomponent) 1.0)))