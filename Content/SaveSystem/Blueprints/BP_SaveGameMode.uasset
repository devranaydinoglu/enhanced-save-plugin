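; BP_SaveGameMode is a game mode that exercises a save system with runtime-spawned actors and a test float.
; On BeginPlay it finds every BP_SavableActor and spawns another beside each, offset along world X with a fixed rotation.
; The PreSaveGame and PostLoadGame events print FloatTest, exposing the game mode's value before saving and after loading.
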(event EventPreSaveGame
  (Development|PrintString (Utilities|String|Append "Game mode FloatTest:" (Utilities|String|ToString(Float) (Variables|Default|GetFloatTest))) true true "(R=0.000000,G=0.660000,B=1.000000,A=1.000000)" 8.0))

(event EventPostLoadGame
  (Development|PrintString (Utilities|String|Append "Game mode FloatTest:" (Utilities|String|ToString(Float) (Variables|Default|GetFloatTest))) true true "(R=0.000000,G=0.660000,B=1.000000,A=1.000000)" 8.0))

(event EventBeginPlay
  (bind _outactors (Actor|GetAllActorsOfClass "/Game/SaveSystem/Blueprints/BP_SavableActor.BP_SavableActor_C"))
  (for _array_element _outactors
    (Game|SpawnActorfromClass "/Game/SaveSystem/Blueprints/BP_SavableActor.BP_SavableActor_C" (Math|Transform|MakeTransform (Math|Vector|MakeVector (+ (.x (Transformation|GetActorLocation _array_element)) 6e+02) (.y (Transformation|GetActorLocation _array_element)) (.z (Transformation|GetActorLocation _array_element))) "0.000000,90.000000,0.000000" "1.000000,1.000000,1.000000") "Undefined" "MultiplyWithRoot" 0 0)))

(fn ConstructionScript)